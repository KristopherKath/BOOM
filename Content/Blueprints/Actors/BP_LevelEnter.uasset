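; BP_LevelEnter is a level entrance trigger that moves a door and activates the stage's enemies when the first-person character overlaps it.
; BeginPlay computes the door's target from an offset, and the CloseDoor timeline lerps from the door's current location toward it.
; Each timeline update, rather than a one-time event, also restarts AI brain logic on every BP_AIBase in EndStageReference's enemy list.
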(event EventBeginPlay
  (Variables|Default|SetNewVector (+ (Transformation|GetActorLocation (Variables|Default|GetDoor)) (Variables|Default|GetChangeVector))))

(event Collision|EventActorBeginOverlap
  (params (OtherActor :type Actor%20Object%20Reference))
  (Utilities|Casting|CastToFirstPersonCharacter OtherActor)
  (bind _alpha (Timeline|CloseDoor Play)
    (:Update
      (Transformation|SetActorLocation (Variables|Default|GetDoor) (Math|Vector|Lerp(Vector) (Transformation|GetActorLocation (Variables|Default|GetDoor)) (Variables|Default|GetNewVector) _alpha) false false)
      (for _array_element (Variables|/Script/BOOM.EndStage|GetEnemies (Variables|Default|GetEndStageReference))
        (bind _asbp_aibase (Utilities|Casting|CastToBP_AIBase _array_element))
        (if (Utilities|IsValid (AI|GetAIController _asbp_aibase))
          (Class|BrainComponent|RestartLogic (Variables|/Script/AIModule.AIController|GetBrainComponent (AI|GetAIController _asbp_aibase))))))))

(event EventTick
  (params (DeltaSeconds :type Float%20%28single-precision%29)))

(fn ConstructionScript)