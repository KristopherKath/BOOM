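; BP_EndStage is an actor that moves a Door once its Enemies array is empty, acting as an end-of-stage gate.
; BeginPlay caches the door's starting location.
; Tick polls the array length and, at zero, plays the Linear0To1 timeline, which lerps the door from that start to an offset set by ChangingVector.
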(event EventBeginPlay
  (Variables|Default|SetInitialPosition (Transformation|GetActorLocation (Variables|Default|GetDoor))))

(event Collision|EventActorBeginOverlap
  (params (OtherActor :type Actor%20Object%20Reference)))

(event EventTick
  (params (DeltaSeconds :type Float%20%28single-precision%29))
  (if (== 0 (Utilities|Array|Length (Variables|Default|GetEnemies)))
    (bind _linearfloattrack (Timeline|Linear%200%20to%201 Play)
      (:Update
        (Transformation|SetActorLocation (Variables|Default|GetDoor) (Math|Vector|Lerp(Vector) (Variables|Default|GetInitialPosition) (+ (Variables|Default|GetInitialPosition) (Variables|Default|GetChangingVector)) _linearfloattrack) false false)))))

(fn ConstructionScript)