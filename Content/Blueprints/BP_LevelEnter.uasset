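; BP_LevelEnter is an overlap-triggered actor that moves a referenced Door, apparently to close it upon level entry.
; BeginPlay stores the target position as the Door's location plus ChangeVector.
; Any actor overlap, with no filter, plays the CloseDoor timeline, whose Alpha lerps the Door toward that target without sweeping.
; Each update lerps from the Door's current location rather than a saved start, so the motion compounds.
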(event EventBeginPlay
  (Variables|Default|SetNewVector (+ (Transformation|GetActorLocation (Variables|Default|GetDoor)) (Variables|Default|GetChangeVector))))

(event Collision|EventActorBeginOverlap
  (params (OtherActor :type Actor%20Object%20Reference))
  (bind _alpha (Timeline|CloseDoor Play)
    (:Update
      (Transformation|SetActorLocation (Variables|Default|GetDoor) (Math|Vector|Lerp(Vector) (Transformation|GetActorLocation (Variables|Default|GetDoor)) (Variables|Default|GetNewVector) _alpha) false false))))

(event EventTick
  (params (DeltaSeconds :type Float%20%28single-precision%29)))

(fn ConstructionScript)