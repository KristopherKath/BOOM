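; Cinematic trigger actor that plays an assigned level sequence once when an actor first overlaps it, then changes a linked goal light.
; An Activated flag guards playback, and the sequence player's OnStop delegate calls ChangeLight on the GoalLight when the cinematic stops.
; Overlaps after activation, or with no valid sequence, skip playback and call ChangeLight immediately.
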(event Custom|OnCinematicStop
  (if (Utilities|IsValid (Variables|Default|GetGoalLight))
    (Default|ChangeLight (Variables|Default|GetGoalLight))))

(event EventBeginPlay)

(event Collision|EventActorBeginOverlap
  (params (OtherActor :type Actor%20Object%20Reference))
  (if (and (not (Variables|Default|GetActivated)) (Utilities|IsValid (Variables|Default|GetSequence)))
    (Variables|Default|SetActivated true)
    (bind _outactor (Sequencer|Player|CreateLevelSequencePlayer (Variables|Default|GetSequence)))
    (Sequencer|Player|Play (Variables|/Script/LevelSequence.LevelSequenceActor|GetSequencePlayer _outactor) :!class /Script/MovieScene.MovieSceneSequencePlayer)
    (EventDispatchers|AssignOnStop (Variables|/Script/LevelSequence.LevelSequenceActor|GetSequencePlayer _outactor) (delegate Custom|OnCinematicStop))
    (elif (Utilities|IsValid (Variables|Default|GetGoalLight))
      (Default|ChangeLight (Variables|Default|GetGoalLight)))))

(fn ConstructionScript)