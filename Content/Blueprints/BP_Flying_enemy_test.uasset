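; BP_Flying_enemy_test is a test enemy that shoots projectiles at the player when its PawnSensing component sees a FirstPersonCharacter.
; Each sighting spawns a FirstPersonProjectile at ProjectileSpawnLocation and launches its mesh with a velocity-change impulse along the Cube's forward vector, scaled by ShootAmount.
; A SpawnProjectile flag with a short delay rate-limits firing.
; The file shows no flight or aiming logic.
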(event OnSeePawn(PawnSensing)
  (params (Pawn :type Pawn%20Object%20Reference))
  ;[1 1 1] Senses Player
  (Utilities|Casting|CastToFirstPersonCharacter Pawn)
  (if (Variables|Default|GetSpawnProjectile)
    (bind _returnvalue (Game|SpawnActorfromClass "/Game/Blueprints/FirstPersonProjectile.FirstPersonProjectile_C" (Transformation|GetWorldTransform (Variables|Default|GetProjectileSpawnLocation)) "Undefined" 0 0))
    (Physics|AddImpulse (Variables|/Game/Blueprints/FirstPersonProjectile.FirstPersonProjectile_C|GetStaticMesh1 _returnvalue) (* (Math|Vector|GetForwardVector (Variables|Default|GetCube)) (Variables|Default|GetShoot%20amount)) "None" true)
    (Variables|Default|SetSpawnProjectile false)
    (Utilities|FlowControl|Delay 0.09)
    (Variables|Default|SetSpawnProjectile true)))

(fn ConstructionScript)