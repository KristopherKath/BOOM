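; BP_Turret is a turret that fires projectiles when it sees the first-person player and can be disabled by damage.
; PawnSensing sightings spawn a projectile at the spawn point and launch it along the Cube's forward vector with a velocity-change impulse.
; A boolean gate reset by a short delay limits the fire rate.
; Damage reduces and prints the Health component's value, and at zero or below a Dead flag stops firing.
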(event OnSeePawn(PawnSensing)
  (params (Pawn :type Pawn%20Object%20Reference))
  ;[1 1 1] Senses Player
  (Utilities|Casting|CastToFirstPersonCharacter Pawn)
  (if (not (Variables|Default|GetDead))
    (if (Variables|Default|GetSpawnProjectile)
      (bind _returnvalue (Game|SpawnActorfromClass "/Game/Blueprints/FirstPersonProjectile.FirstPersonProjectile_C" (Transformation|GetWorldTransform (Variables|Default|GetProjectileSpawnLocation)) "Undefined" 0 0))
      (Physics|AddImpulse (Variables|/Game/Blueprints/FirstPersonProjectile.FirstPersonProjectile_C|GetStaticMesh1 _returnvalue) (* (Math|Vector|GetForwardVector (Variables|Default|GetCube)) (Variables|Default|GetShoot%20amount)) "None" true)
      (Variables|Default|SetSpawnProjectile false)
      (Utilities|FlowControl|Delay 0.09)
      (Variables|Default|SetSpawnProjectile true))))

(event Game|Damage|EventAnyDamage
  (params (Damage :type Float%20%28single-precision%29) (DamageType :type Damage%20Type%20Object%20Reference) (InstigatedBy :type Controller%20Object%20Reference) (DamageCauser :type Actor%20Object%20Reference))
  (bind _output_get (Variables|/Script/BOOM.Health|SetHealth (Variables|Default|GetHealth) (- (Variables|/Script/BOOM.Health|GetHealth (Variables|Default|GetHealth)) Damage)))
  (Development|PrintString (Utilities|String|ToString(Float) _output_get))
  (if (<= (Variables|/Script/BOOM.Health|GetHealth (Variables|Default|GetHealth)) 0.0)
    (Variables|Default|SetDead true)))

(fn ConstructionScript)