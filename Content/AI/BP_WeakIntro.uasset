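; BP_WeakIntro is an AI character with health and a melee attack, whose AI brain logic is stopped on BeginPlay.
; A custom event plays the Melee_Attack montage.
; Damage lowers the Health component's value; at zero it sets Dead, stops the brain and disables capsule collision.
; Tick sets Speed to a fixed value from whether it moves and copies the Normal_AI blackboard's PlayerinMeleeRange flag into CanAttack.
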(event Custom|CustomEvent
  (Animation|Montage|PlayMontage (Variables|Character|GetMesh) "/Game/Animations/TheWeak/Melee_Attack.Melee_Attack"))

(event Game|Damage|EventAnyDamage
  (params (Damage :type Float%20%28single-precision%29) (DamageType :type Damage%20Type%20Object%20Reference) (InstigatedBy :type Controller%20Object%20Reference) (DamageCauser :type Actor%20Object%20Reference))
  (bind _output_get (Variables|/Script/BOOM.Health|SetHealth (Variables|Default|GetHealth) (- (Variables|/Script/BOOM.Health|GetHealth (Variables|Default|GetHealth)) Damage)))
  (Development|PrintString (Utilities|String|ToString(Float) _output_get))
  (if (<= (Variables|/Script/BOOM.Health|GetHealth (Variables|Default|GetHealth)) 0.0)
    (Variables|Default|SetDead true)
    (AI|Logic|StopLogic (Variables|/Script/AIModule.AIController|GetBrainComponent (AI|GetAIController self)) "")
    (Collision|SetCollisionEnabled (Variables|Default|GetCapsuleComponent) "NoCollision")))

(event EventTick
  (params (DeltaSeconds :type Float%20%28single-precision%29))
  (if (> (Math|Vector|VectorLength (Transformation|GetVelocity)) 0.0)
    (Variables|Default|SetSpeed 1e+02)
    (else
      (Variables|Default|SetSpeed 0.0)))
  (bind _asnormal_ai (Utilities|Casting|CastToNormal_AI (AI|GetAIController 0)))
  (Variables|Default|SetCanAttack (ScalableFloat|GetValueasBool (AI|GetBlackboard _asnormal_ai) (Utilities|Name|MakeLiteralName "PlayerinMeleeRange"))))

(event EventBeginPlay
  (AI|Logic|StopLogic (Variables|/Script/AIModule.AIController|GetBrainComponent (AI|GetAIController self)) ""))

(fn ConstructionScript
  (|CallParentFunction))